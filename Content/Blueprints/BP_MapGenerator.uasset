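; BP_MapGenerator builds a blocky voxel terrain from spawned cube actors when play begins.
; GenerateWorld loops over the X/Y map grid and stacks a random-height column of scaled cubes in each cell, independent of its neighbors.
; GetBlockType maps each cube's height index to rock, grass or snow using threshold heights, and the matching material is applied to the cube's root mesh.
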(event EventBeginPlay
  (CallFunction|GenerateWorld))

(event EventTick
  (params (DeltaSeconds :type Float%20%28single-precision%29)))

(fn ConstructionScript)

(fn GenerateWorld
  ;[1 1 1] Calculate the final size
  (LocalVariables|SetCubeBrickFinalSize (* (Variables|Default|GetCubeBrickScale) (Variables|Default|GetCubeBrickSize)))
  ;[1 1 1] Calculate IDs and Bricks centers
  (for _index (range 0 (Math|Float|Truncate (.x (Variables|Default|GetMapSize))))
    (LocalVariables|SetxID _index)
    (for _index_2 (range 0 (Math|Float|Truncate (.y (Variables|Default|GetMapSize))))
      (LocalVariables|SetyID _index_2)
      (for _index_3 (range 0 (Math|Random|RandomIntegerinRange 6 35))
        (LocalVariables|SetzID _index_3)
        ;[1 1 1] Spawn Cube bricks
        (bind _returnvalue (Game|SpawnActorfromClass (Variables|Default|GetCubeClass) (Math|Transform|MakeTransform (Math|Vector|MakeVector (* (LocalVariables|GetxID) (.x (LocalVariables|GetCubeBrickFinalSize))) (* (LocalVariables|GetyID) (.y (LocalVariables|GetCubeBrickFinalSize))) (* (LocalVariables|GetzID) (.z (LocalVariables|GetCubeBrickFinalSize)))) "0, 0, 0" (Variables|Default|GetCubeBrickScale)) "Undefined" "MultiplyWithRoot" 0 0))
        ;[1 1 1] Check validation
        (bind _output_get (LocalVariables|SetSpawnedBrick _returnvalue))
        (Utilities|IsValid _output_get
          (:Is%20Valid
            (bind _returnvalue_2 (CallFunction|GetBlockType (LocalVariables|GetzID)))
            (bind _asmesh_component (Utilities|Casting|CastToMeshComponent (Variables|/Script/Engine.Actor|GetRootComponent (LocalVariables|GetSpawnedBrick))))
            (Rendering|Material|SetMaterial _asmesh_component 0 (Utilities|Select :Index _returnvalue_2 :NewEnumerator0 (Variables|Default|GetRockMaterial) :NewEnumerator1 (Variables|Default|GetGrassMaterial) :NewEnumerator2 (Variables|Default|GetSnowMaterial))))
          (:Is%20Not%20Valid
            (Development|PrintString (Utilities|String|Append "Error: Failed to spawn the CubeBirck id=" (Utilities|String|Append "(" (Utilities|String|ToString(Integer) (LocalVariables|GetxID)) ", " (Utilities|String|ToString(Integer) (LocalVariables|GetyID)) ", " (Utilities|String|ToString(Integer) (LocalVariables|GetzID)) ")")))))))))

(fn GetBlockType
  (params (GridZ :type Integer))
  (if (< GridZ (Variables|Default|GetGrassStartHeight))
    (return "NewEnumerator0")
    (elif (< GridZ (Variables|Default|GetSnowStartHeight))
      (return "NewEnumerator1")
      (else
        (return "NewEnumerator2")))))