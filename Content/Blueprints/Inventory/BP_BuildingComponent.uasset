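; Building component that places voxel blocks at hit locations and tracks the active block type.
; Placement offsets the impact point along the surface normal, then asks the voxel world subsystem to place the block, broadcasting on success, or snap it for a placement location.
; Block order comes from the voxel definition subsystem; cycling wraps around it and broadcasts each selection change.
; The initial type is selected by index once definitions are ready.
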(event EventBeginPlay
  (EventDispatchers|AssignOnDefinitionsReady (Subsystems|GetVoxelDefinitionSubsystem) (EventDispatchers|CreateEvent :!event OnDefinitionsReady)))

(fn ProcessBuilding
  (params (HitResult :type Hit%20Result%20Structure))
  (bind _returnvalue (Subsystems|GetVoxelWorldSubsystem))
  (if (.bBlockingHit (Collision|BreakHitResult HitResult))
    (bind _returnvalue_2 (Class|VoxelWorldSubsystem|TryPlaceBlock _returnvalue (Class|VoxelWorldSubsystem|BlockWorldLocationtoGlobalPosition _returnvalue (CallFunction|GetHitPointLocation HitResult)) (Variables|Default|GetActiveBuildingBlockType)))
    (if _returnvalue_2
      (Default|CallOnBlockBuilt (Variables|Default|GetActiveBuildingBlockType))
      (return true)
      (else
        (return false)))
    (else
      (return false))))

(fn CycleActiveBuildingBlockType
  (params (Direction :type Integer))
  (bind _returnvalue (CallFunction|GetBuildingBlockTypesOrder))
  (bind _returnvalue_2 (Utilities|Array|Length _returnvalue))
  (if (Utilities|Array|IsEmpty (CallFunction|GetBuildingBlockTypesOrder))
    (return)
    (else
      (LocalVariables|SetNextIndex (Math|Integer|%(Integer) (+ (+ Direction (Variables|Default|GetActiveBuildingBlockTypeIndex)) _returnvalue_2) _returnvalue_2))
      (LocalVariables|SetPreviousBlockType (Variables|Default|GetActiveBuildingBlockType))
      (CallFunction|SetActiveBuildingBlockTypebyIndex (LocalVariables|GetNextIndex))
      (return))))

(fn SetActiveBuildingBlockTypebyIndex
  (params (Index :type Integer))
  (LocalVariables|SetPreviousBlockType (Variables|Default|GetActiveBuildingBlockType))
  (Variables|Default|SetActiveBuildingBlockType (Utilities|Array|Get(acopy) (CallFunction|GetBuildingBlockTypesOrder) Index))
  (Variables|Default|SetActiveBuildingBlockTypeIndex Index)
  (Default|CallOnActiveBuildingBlockTypeChanged (LocalVariables|GetPreviousBlockType) (Variables|Default|GetActiveBuildingBlockType))
  (return))

(fn GetBuildingBlockTypesOrder
  (return (Class|VoxelDefinitionSubsystem|GetBuildingBlockTypeOrder (Subsystems|GetVoxelDefinitionSubsystem))))

(fn GetActiveBuildingBlockType
  (return (Variables|Default|GetActiveBuildingBlockType)))

(fn OnDefinitionsReady
  (CallFunction|SetActiveBuildingBlockTypebyIndex 1))

(fn GetPlacementWorldLocation
  (params (Hit :type Hit%20Result%20Structure%20%28by%20ref%29))
  (return (Class|VoxelWorldSubsystem|SnapWorldLocationtoBlockOrigin (Subsystems|GetVoxelWorldSubsystem) (CallFunction|GetHitPointLocation Hit))))

(fn GetHitPointLocation
  (params (Hit :type Hit%20Result%20Structure%20%28by%20ref%29))
  (bind (_bblockinghit _binitialoverlap _time _distance _location _impactpoint _normal _impactnormal) (Collision|BreakHitResult Hit))
  (return (+ _impactpoint (* _impactnormal (Variables|Default|GetTraceEndOffset)))))