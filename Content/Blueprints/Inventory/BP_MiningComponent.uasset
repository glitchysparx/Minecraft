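; Mining component that breaks voxel world blocks after sustained targeting for a duration looked up by block type.
; ProcessMining takes a hit result and delta time, steps inside the surface to resolve the block, and resets the timer when the target changes or is lost.
; It broadcasts progress, then has VoxelWorldSubsystem destroy the block and announces success.
; StartMining and StopMining both broadcast a false mining state; only Stop clears the target.
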(event EventBeginPlay)

(event EventTick
  (params (DeltaSeconds :type Float%20%28single-precision%29)))

(fn StartMining
  (Default|CallOnMiningStateChanged false)
  (return))

(fn StopMining
  (Helpers|ClearMiningTarget)
  (Default|CallOnMiningStateChanged false)
  (return))

(fn ProcessMining
  (params (HitResult :type Hit%20Result%20Structure%20%28by%20ref%29) (DeltaSeconds :type Float%20%28double-precision%29))
  (bind _output_get (LocalVariables|SetTraceHitResult HitResult))
  (if (.bBlockingHit (Collision|BreakHitResult _output_get))
    (LocalVariables|SetTargetHitLocation (- (.ImpactPoint (Collision|BreakHitResult (LocalVariables|GetTraceHitResult))) (* (.ImpactNormal (Collision|BreakHitResult (LocalVariables|GetTraceHitResult))) (Variables|Default|GetTraceEndOffset))))
    (Utilities|Casting|CastToVoxelChunk (.HitActor (Collision|BreakHitResult (LocalVariables|GetTraceHitResult)))
      (:then
        (bind _output_get_2 (LocalVariables|SetHitBlockPosition (Class|VoxelWorldSubsystem|BlockWorldLocationtoGlobalPosition (Subsystems|GetVoxelWorldSubsystem) (LocalVariables|GetTargetHitLocation))))
        (if (Helpers|IsNewMiningTarget _output_get_2)
          (Helpers|TrySetMiningTarget (LocalVariables|GetHitBlockPosition))
          (return)
          (else
            (bind _output_get_3 (Variables|Default|SetElapsedMiningTime (+ (Variables|Default|GetElapsedMiningTime) DeltaSeconds)))
            (if (>= _output_get_3 (Variables|Default|GetRequiredMiningTime))
              (bind _returnvalue (Class|VoxelWorldSubsystem|TryDestroyBlockfromHit (Subsystems|GetVoxelWorldSubsystem) (LocalVariables|GetTraceHitResult) (Variables|Default|GetTraceEndOffset)))
              (if _returnvalue
                (Default|CallOnBlockMined (Variables|Default|GetMiningTargetBlockType)))
              (Helpers|ClearMiningTarget)
              (return)
              (else
                (Default|CallOnMiningProgressChanged (/ (Variables|Default|GetElapsedMiningTime) (Variables|Default|GetRequiredMiningTime)))
                (return))))))
      (:CastFailed
        (Helpers|ClearMiningTarget)
        (return)))
    (else
      (Helpers|ClearMiningTarget)
      (return))))

(fn ClearMiningTarget
  (Variables|Default|SetHasMiningTarget false)
  (Variables|Default|SetElapsedMiningTime 0.0)
  (Default|CallOnMiningProgressChanged 0.0)
  (return))

(fn IsNewMiningTarget
  (params (BlockIndexToCheck :type Int%20Vector%20Structure))
  (bind _miningtargetblock (Variables|Default|GetMiningTargetBlock))
  (return (or (not (Variables|Default|GetHasMiningTarget)) (not (Math|Boolean|ANDBoolean (== (.x _miningtargetblock) (.x BlockIndexToCheck)) (== (.y _miningtargetblock) (.y BlockIndexToCheck)) (== (.z _miningtargetblock) (.z BlockIndexToCheck)))))))

(fn TrySetMiningTarget
  (params (NewTargetBlockIndex :type Int%20Vector%20Structure))
  (bind (_voxelblock _returnvalue) (Class|VoxelWorldSubsystem|GetBlockatGlobalPosition (Subsystems|GetVoxelWorldSubsystem) NewTargetBlockIndex))
  (Variables|Default|SetMiningTargetBlockType (.type _voxelblock))
  (if _returnvalue
    (Variables|Default|SetMiningTargetBlock NewTargetBlockIndex)
    (Variables|Default|SetHasMiningTarget true)
    (Variables|Default|SetElapsedMiningTime 0.0)
    (Variables|Default|SetRequiredMiningTime (.TimeValue (Helpers|GetMiningDuration (Variables|Default|GetMiningTargetBlockType))))
    (return)
    (else
      (Development|PrintString (Utilities|String|Append "Unexpected error occured while trying to find a Block on Position: " (Utilities|String|ToString(Integer) NewTargetBlockIndex)) false)
      (return))))

(fn GetMiningDuration
  (params (BlockType :type EVoxelBlockType%20Enum :default "Air"))
  (bind _miningduration (Variables|Default|GetMiningDuration))
  (bind (_value _returnvalue) (Utilities|Map|Find _miningduration BlockType))
  (return _value _returnvalue))