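; Inventory component that stores resource amounts in a map keyed by resource type.
; AddResource accepts positive amounts, while TryConsumeResource checks availability before subtracting and removes entries that reach zero.
; Successful changes fire OnInventoryChanged with the type and new amount, and GetAllResources exposes the map.
; TryConsumeResource returns true even when the availability check fails, so its result does not signal failure.
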(event EventBeginPlay)

(event EventTick
  (params (DeltaSeconds :type Float%20%28single-precision%29)))

(fn AddResource
  (params (Type :type EResourceType%20Enum :default "None") (Amount :type Integer))
  (if (> Amount 0)
    (bind _output_get (LocalVariables|SetCombinedAmount (+ (.Value (Utilities|Map|Find (Variables|Inventory|Resources|GetResources) Type)) Amount)))
    (Utilities|Map|Add (Variables|Inventory|Resources|GetResources) Type _output_get)
    (Default|CallOnInventoryChanged Type (LocalVariables|GetCombinedAmount))
    (return true)
    (else
      (Development|PrintString "Incorrect amount of resources!" false)
      (return false))))

(fn TryConsumeResource
  (params (Type :type EResourceType%20Enum%20%28by%20ref%29 :default "None") (Amount :type Integer))
  (bind _result (CallFunction|CheckResourceAvailability Type Amount))
  (if _result
    (bind _output_get (LocalVariables|SetTargetAmount (- (.Value (Utilities|Map|Find (Variables|Inventory|Resources|GetResources) Type)) Amount)))
    (if (== _output_get 0)
      (Utilities|Map|Remove (Variables|Inventory|Resources|GetResources) Type)
      (else
        (Utilities|Map|Add (Variables|Inventory|Resources|GetResources) Type (LocalVariables|GetTargetAmount))))
    (Default|CallOnInventoryChanged Type (LocalVariables|GetTargetAmount))
    (return true)
    (else
      (return true))))

(fn GetAllResources
  (return (Variables|Inventory|Resources|GetResources)))

(fn CheckResourceAvailability
  (params (Type :type EResourceType%20Enum%20%28by%20ref%29 :default "None") (Amount :type Integer))
  (bind _resources (Variables|Inventory|Resources|GetResources))
  (bind (_value _returnvalue) (Utilities|Map|Find _resources Type))
  (LocalVariables|SetTotalAmount _value)
  (if _returnvalue
    (if (and (> (LocalVariables|GetTotalAmount) 0) (> Amount 0))
      (return (>= (LocalVariables|GetTotalAmount) Amount))
      (else
        (return false)))
    (else
      (return false))))