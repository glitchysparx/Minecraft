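; BP_VoxelChunk is one chunk of a voxel world, generating noise-based rock, grass and snow terrain and supporting runtime block edits.
; A batched state machine fills block data, finds air-exposed blocks, then adds them to per-type instanced meshes.
; Edits flag changes and refresh the block and its neighbours, finding instances by hit index or location search.
; Applying saved modification deltas is unfinished: the loop is empty and the merge call is unreachable.
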(fn ConstructionScript)

(fn AddPendingBlock
  (params (Index :type Integer) (LocalGridPosition :type Int%20Vector%20Structure%20%28by%20ref%29) (Type :type EVoxelBlockType%20Enum :default "Air"))
  (Utilities|Array|Add (Variables|Default|GetPendingBlocks) (Utilities|Struct|MakePendingBlockInstance Index (Class|VoxelChunk|MakeBlockLocalTransform LocalGridPosition) Type))
  (return))

(fn DetermineTerrainBlockType
  (params (GridZ :type Integer))
  (if (< GridZ (Variables|VoxelChunk|Constants|GetGrassStartHeight))
    (return "Rock")
    (elif (< GridZ (Variables|VoxelChunk|Constants|GetSnowStartHeight))
      (return "Grass")
      (else
        (return "Snow")))))

(fn GenerateChunkData
  (params (BatchSize :type Integer))
  (bind _chunkheightrange (Variables|VoxelChunk|ChunkData|GetChunkHeightRange))
  (bind _output_get (LocalVariables|SetCount (Math|Integer|Max(Integer) (Math|Integer|Min(Integer) (- (VoxelChunk|ChunkData|GetTotalBlocksCount) (Variables|Default|Cache|GetDataGenerationIndex)) BatchSize))))
  (bind _output_get_2 (LocalVariables|SetEndExlusive (+ _output_get (Variables|Default|Cache|GetDataGenerationIndex))))
  (for _index (range (Variables|Default|Cache|GetDataGenerationIndex) (- _output_get_2 1))
    (bind _output_get_3 (LocalVariables|SetLocalPosition (Class|WorldGenerationFunctionLibrary|BlockIndextoLocalGridPosition _index (CallFunction|GetChunkSize3D))))
    (bind _output_get_4 (LocalVariables|SetGlobalPosition (Class|WorldGenerationFunctionLibrary|BlockLocalPositiontoGlobal _output_get_3 (CallFunction|GetChunkSize3D) (Class|VoxelChunk|GetChunkIndex))))
    (bind _output_get_5 (LocalVariables|SetTerrainHeight (Class|WorldGenerationFunctionLibrary|CalculateTerrainHeight (.x _output_get_4) (.y _output_get_4) (Variables|VoxelChunk|ChunkData|GetNoiseFrequency) (Variables|VoxelChunk|ChunkData|GetNoiseOffset) (.x _chunkheightrange) (.y _chunkheightrange))))
    (if (>= _output_get_5 (.z (LocalVariables|GetGlobalPosition)))
      (bind _returnvalue (VoxelChunk|Generation|Steps|Helpers|DetermineTerrainBlockType (.z (LocalVariables|GetGlobalPosition))))
      (LocalVariables|SetBlockType _returnvalue)
      (else
        (LocalVariables|SetBlockType "Air")))
    (VoxelChunk|Generation|Steps|Helpers|RegisterBlockbyPosition (LocalVariables|GetBlockType) (LocalVariables|GetLocalPosition)))
  (bind _output_get_6 (Variables|Default|Cache|SetDataGenerationIndex (LocalVariables|GetEndExlusive)))
  (return (== _output_get_6 (VoxelChunk|ChunkData|GetTotalBlocksCount))))

(fn BuildNextBatch
  (params (BatchSize :type Integer))
  (if (VoxelChunk|Generation|Steps|Helpers|IsBuildFinished)
    (return true)
    (else
      (LocalVariables|SetRemaining BatchSize)
      (bind (_nextindex _addedcount) (VoxelChunk|Generation|Steps|Helpers|BuildTypeBatch (Variables|Default|GetPendingBlocks) (Variables|Default|Cache|GetDataGenerationIndex) (LocalVariables|GetRemaining)))
      (Variables|Default|Cache|SetDataGenerationIndex _nextindex)
      (LocalVariables|SetRemaining (- (LocalVariables|GetRemaining) _addedcount))
      (return (VoxelChunk|Generation|Steps|Helpers|IsBuildFinished)))))

(fn BuildTypeBatch
  (params (PendingBlocks :type Array%20of%20Pending%20Block%20Instance%20Structures) (StartIndex :type Integer) (MaxCount :type Integer))
  (if (Math|Boolean|ANDBoolean (>= StartIndex 0) (< StartIndex (Utilities|Array|Length PendingBlocks)) (> MaxCount 0))
    (LocalVariables|SetCount (Math|Integer|Min(Integer) (- (Utilities|Array|Length PendingBlocks) StartIndex) MaxCount))
    (for _index (range StartIndex (- (+ StartIndex (LocalVariables|GetCount)) 1))
      (bind _output_get (LocalVariables|SetNextPendingBlock (Utilities|Array|Get(acopy) PendingBlocks _index)))
      (if (Utilities|Enum|Equal(Enum) (.Type (Utilities|Struct|BreakPendingBlockInstance _output_get)) (LocalVariables|GetBlockType))
        _
        (else
          (bind _output_get_2 (LocalVariables|SetInstanceMeshComponent (VoxelChunk|Generation|Steps|Helpers|GetInstMeshComponentbyType (.type (LocalVariables|GetPendingBlock)))))
          (Utilities|IsValid _output_get_2
            (:Is%20Valid
              (Components|InstancedStaticMesh|AddInstances (LocalVariables|GetInstanceMeshComponent) (LocalVariables|GetBatch) false false true))
            (:Is%20Not%20Valid
              _))
          (LocalVariables|SetBlockType (.type (LocalVariables|GetNextPendingBlock)))
          (Utilities|Array|Clear (LocalVariables|GetBatch))))
      (bind _output_get_3 (LocalVariables|SetPendingBlock (LocalVariables|GetNextPendingBlock)))
      (Utilities|Array|Add (LocalVariables|GetBatch) (.transform _output_get_3))
      (Utilities|Struct|SetmembersinVoxelBlock (Utilities|Array|Get(acopy) (Variables|Default|GetBlocks) (.blockindex (LocalVariables|GetPendingBlock))) true))
    (bind _output_get_4 (LocalVariables|SetInstanceMeshComponent (VoxelChunk|Generation|Steps|Helpers|GetInstMeshComponentbyType (.type (LocalVariables|GetPendingBlock)))))
    (Utilities|IsValid _output_get_4
      (:Is%20Valid
        (Components|InstancedStaticMesh|AddInstances (LocalVariables|GetInstanceMeshComponent) (LocalVariables|GetBatch) false false true))
      (:Is%20Not%20Valid
        _))
    (return (+ StartIndex (LocalVariables|GetCount)) (LocalVariables|GetCount))
    (else
      (return StartIndex 0))))

(fn IsBuildFinished
  (return (>= (Variables|Default|Cache|GetDataGenerationIndex) (Utilities|Array|Length (Variables|Default|GetPendingBlocks)))))

(fn ClearCache
  (Utilities|Array|Clear (Variables|Default|GetPendingBlocks))
  (Variables|Default|Cache|SetDataGenerationIndex 0)
  (return))

(fn RegisterBlockbyPosition
  (params (Type :type EVoxelBlockType%20Enum :default "Air") (LocalGridPosition :type Int%20Vector%20Structure%20%28by%20ref%29))
  (VoxelChunk|Generation|Steps|Helpers|RegisterBlockbyIndex Type (Class|WorldGenerationFunctionLibrary|BlockLocalGridPositiontoIndex LocalGridPosition (CallFunction|GetChunkSize3D)))
  (return))

(fn FindExposedBlocks
  (params (BatchSize :type Integer))
  (bind _output_get (LocalVariables|SetCount (Math|Integer|Max(Integer) (Math|Integer|Min(Integer) (- (VoxelChunk|ChunkData|GetTotalBlocksCount) (Variables|Default|Cache|GetDataGenerationIndex)) BatchSize))))
  (bind _output_get_2 (LocalVariables|SetEndExlusive (+ _output_get (Variables|Default|Cache|GetDataGenerationIndex))))
  (for _index (range (Variables|Default|Cache|GetDataGenerationIndex) (- _output_get_2 1))
    (bind _output_get_3 (LocalVariables|SetBlockIndex _index))
    (bind _output_get_4 (LocalVariables|SetBlockType (.type (Utilities|Array|Get(acopy) (Variables|Default|GetBlocks) _output_get_3))))
    (if (not (Utilities|Enum|Equal(Enum) _output_get_4 "Air"))
      (bind _output_get_5 (LocalVariables|SetBlockLocalGridPosition (Class|WorldGenerationFunctionLibrary|BlockIndextoLocalGridPosition (LocalVariables|GetBlockIndex) (CallFunction|GetChunkSize3D))))
      (bind _returnvalue (VoxelChunk|Editing|Helpers|IsBlockExposed _output_get_5))
      (if _returnvalue
        (VoxelChunk|Generation|Steps|Helpers|AddPendingBlock (LocalVariables|GetBlockIndex) (LocalVariables|GetBlockLocalGridPosition) (LocalVariables|GetBlockType)))))
  (bind _output_get_6 (Variables|Default|Cache|SetDataGenerationIndex (LocalVariables|GetEndExlusive)))
  (return (== _output_get_6 (VoxelChunk|ChunkData|GetTotalBlocksCount))))

(fn IsBlockExposed
  (params (LocalGridPosition :type Int%20Vector%20Structure))
  (bind _array_element (Utilities|Array|ForEachLoopwithBreak (Variables|VoxelChunk|Constants|GetNeighbouringDirections))
    (:LoopBody
      (bind _returnvalue (VoxelChunk|Editing|Helpers|GetNeighbourBlockType LocalGridPosition _array_element))
      (if (Utilities|Enum|Equal(Enum) _returnvalue "Air")
        (return true)))
    (:Completed
      (return false))))

(fn GetNeighbourBlockType
  (params (LocalGridPosition :type Int%20Vector%20Structure) (Direction :type Int%20Vector%20Structure))
  (bind _returnvalue (CallFunction|GetChunkSize3D))
  (bind _output_get (LocalVariables|SetNeighbourPosition (Utilities|Struct|MakeIntVector (+ (.x LocalGridPosition) (.x Direction)) (+ (.y LocalGridPosition) (.y Direction)) (+ (.z LocalGridPosition) (.z Direction)))))
  (if (Math|Boolean|ANDBoolean (Math|Integer|InRange(Integer) (.X (Utilities|Struct|BreakIntVector _output_get)) 0 (.x _returnvalue) true false) (Math|Integer|InRange(Integer) (.Y (Utilities|Struct|BreakIntVector _output_get)) 0 (.y _returnvalue) true false) (Math|Integer|InRange(Integer) (.Z (Utilities|Struct|BreakIntVector _output_get)) 0 (.z _returnvalue) true false))
    (return (.type (Utilities|Array|Get(acopy) (Variables|Default|GetBlocks) (Class|WorldGenerationFunctionLibrary|BlockLocalGridPositiontoIndex (LocalVariables|GetNeighbourPosition) (CallFunction|GetChunkSize3D)))) true)
    (else
      (return "Air" true))))

(fn GetTotalBlocksCount
  (return (Utilities|Array|Length (Variables|Default|GetBlocks))))

(fn ProcessGenerationStep
  (params (BatchSize :type Integer))
  (switch Utilities|FlowControl|Switch|SwitchonEChunkGenerationState (Class|VoxelChunk|GetGenerationState)
    (:Pending
      _)
    (:GenerateData
      _)
    (:FindExposedBlocks
      (bind _finished (VoxelChunk|Generation|Steps|FindExposedBlocks BatchSize))
      (if _finished
        (Class|VoxelChunk|SetGenerationState "BuildingInstances")
        (Variables|Default|Cache|SetDataGenerationIndex 0))
      (return false))
    (:BuildingInstances
      (bind _finished_2 (VoxelChunk|Generation|Steps|BuildNextBatch BatchSize))
      (if _finished_2
        (Class|VoxelChunk|SetGenerationState "Completed")
        (VoxelChunk|Generation|ClearCache))
      (return false))
    (:Completed
      (return (Class|VoxelChunk|IsGenerationComplete))))
  (bind _finished_3 (VoxelChunk|Generation|Steps|GenerateChunkData BatchSize))
  (if _finished_3
    (Class|VoxelChunk|SetGenerationState "FindExposedBlocks")
    (Variables|Default|Cache|SetDataGenerationIndex 0))
  (return false))

(fn InitializeChunk
  (params (NewIndex :type Int%20Vector%20Structure) (NewSize :type Int%20Point%20Structure) (NewHeightRange :type Int%20Point%20Structure) (NewNoiseOffset :type Vector%202D%20Structure) (NewNoiseFrequency :type Float%20%28single-precision%29) (NewBlockScale :type Vector :default "0, 0, 0") (NewBlockSize :type Vector :default "0, 0, 0"))
  (if (Variables|Default|Cache|GetIsInitialized)
    (return false)
    (else
      (Variables|Default|Cache|SetIsInitialized true)
      (Class|VoxelChunk|SetGenerationState "Empty")
      (Variables|Default|SetChunkIndex NewIndex)
      (Variables|VoxelChunk|ChunkData|SetChunkSize2D NewSize)
      (Variables|VoxelChunk|ChunkData|SetChunkHeightRange NewHeightRange)
      (Variables|VoxelChunk|ChunkData|SetNoiseOffset NewNoiseOffset)
      (Variables|VoxelChunk|ChunkData|SetNoiseFrequency NewNoiseFrequency)
      (Variables|Default|SetBlockScale NewBlockScale)
      (Variables|Default|SetBlockSize NewBlockSize)
      (VoxelChunk|Generation|ClearCache)
      (Utilities|Array|Clear (Variables|Default|GetBlocks))
      (Utilities|Array|Resize (Variables|Default|GetBlocks) (* (.x (Variables|VoxelChunk|ChunkData|GetChunkSize2D)) (.y (Variables|VoxelChunk|ChunkData|GetChunkSize2D)) (.y (Variables|VoxelChunk|ChunkData|GetChunkHeightRange))))
      (return true))))

(fn GetBlockatLocalPosition
  (params (LocalPosition :type Int%20Vector%20Structure))
  (bind _output_get (LocalVariables|SetTargetIndex (Class|WorldGenerationFunctionLibrary|BlockLocalGridPositiontoIndex LocalPosition (CallFunction|GetChunkSize3D))))
  (if (< _output_get (VoxelChunk|ChunkData|GetTotalBlocksCount))
    (return (Utilities|Array|Get(acopy) (Variables|Default|GetBlocks) (LocalVariables|GetTargetIndex)) (LocalVariables|GetTargetIndex) true)
    (else
      (return "" 0 false))))

(fn SetBlockatLocalPosition
  (params (LocalPosition :type Int%20Vector%20Structure) (NewType :type EVoxelBlockType%20Enum :default "Air"))
  (bind _returnvalue (CallFunction|SetBlockatLocalPositionwithInstanceHint LocalPosition NewType -1))
  (return _returnvalue))

(fn RefreshBlockVisual
  (params (LocalPosition :type Int%20Vector%20Structure))
  (bind (_voxelblock _localblockindex _returnvalue) (CallFunction|GetBlockatLocalPosition LocalPosition))
  (LocalVariables|SetVoxelBlock _voxelblock)
  (LocalVariables|SetBlockIndex _localblockindex)
  (if _returnvalue
    (if (Utilities|Enum|Equal(Enum) (.type (LocalVariables|GetVoxelBlock)) "Air")
      (return true)
      (else
        (bind _returnvalue_2 (VoxelChunk|Editing|Helpers|IsBlockExposed LocalPosition))
        (if _returnvalue_2
          (if (.bhasinstance (LocalVariables|GetVoxelBlock))
            (return true)
            (else
              (VoxelChunk|Editing|Helpers|AddBlockInstance (LocalVariables|GetBlockIndex))
              (return true)))
          (elif (.bhasinstance (LocalVariables|GetVoxelBlock))
            (VoxelChunk|Editing|Helpers|RemoveBlockInstance (LocalVariables|GetBlockIndex) -1)
            (return true)
            (else
              (return true))))))
    (else
      (return false))))

(fn RemoveBlockInstance
  (params (BlockIndex :type Integer) (BlockInstanceIndexHint :type Integer))
  (if (< BlockIndex (VoxelChunk|ChunkData|GetTotalBlocksCount))
    (LocalVariables|SetBlock (Utilities|Array|Get(acopy) (Variables|Default|GetBlocks) BlockIndex))
    (if (.bhasinstance (LocalVariables|GetBlock))
      (LocalVariables|SetTargetISM (VoxelChunk|Generation|Steps|Helpers|GetInstMeshComponentbyType (.type (LocalVariables|GetBlock))))
      (if (>= BlockInstanceIndexHint 0)
        ;[1 1 1] Line traces read the instance index and store it in Hit.Item value
        (LocalVariables|SetBlockInstanceIndex BlockInstanceIndexHint)
        (else
          ;[1 1 1] Linear search to find the target instance. Caching instances would not work because they are changing after remove/add operations
          (LocalVariables|SetBlockInstanceIndex (Class|WorldGenerationFunctionLibrary|FindBlockInstanceIndexbyLocation (LocalVariables|GetTargetISM) (Class|WorldGenerationFunctionLibrary|BlockLocalPositiontoChunkLocalLocation (Class|WorldGenerationFunctionLibrary|BlockIndextoLocalGridPosition BlockIndex (CallFunction|GetChunkSize3D)) (Variables|Default|GetBlockSize) (Variables|Default|GetBlockScale)) false))))
      (Utilities|IsValid (LocalVariables|GetTargetISM)
        (:Is%20Valid
          (Class|InstancedStaticMeshComponent|RemoveInstance (LocalVariables|GetTargetISM) (LocalVariables|GetBlockInstanceIndex)))
        (:Is%20Not%20Valid
          _))
      (bind _structout (Utilities|Struct|SetmembersinVoxelBlock (LocalVariables|GetBlock) false))
      (Utilities|Array|SetArrayElem (Variables|Default|GetBlocks) BlockIndex _structout)
      (return)
      (else
        (return)))
    (else
      (return))))

(fn AddBlockInstance
  (params (BlockIndex :type Integer))
  (if (< BlockIndex (VoxelChunk|ChunkData|GetTotalBlocksCount))
    (LocalVariables|SetBlock (Utilities|Array|Get(acopy) (Variables|Default|GetBlocks) BlockIndex))
    (bind _output_get (LocalVariables|SetTargetISM (VoxelChunk|Generation|Steps|Helpers|GetInstMeshComponentbyType (.type (LocalVariables|GetBlock)))))
    (Utilities|IsValid _output_get
      (:Is%20Valid
        (Components|InstancedStaticMesh|AddInstance (LocalVariables|GetTargetISM) (Class|VoxelChunk|MakeBlockLocalTransform (Class|WorldGenerationFunctionLibrary|BlockIndextoLocalGridPosition BlockIndex (CallFunction|GetChunkSize3D))) false)
        (bind _structout (Utilities|Struct|SetmembersinVoxelBlock (LocalVariables|GetBlock) true))
        (Utilities|Array|SetArrayElem (Variables|Default|GetBlocks) BlockIndex _structout)
        (return))
      (:Is%20Not%20Valid
        (return)))
    (else
      (return))))

(fn RefreshNeighbourBlock
  (params (LocalPosition :type Int%20Vector%20Structure) (NeighbourDirection :type Int%20Vector%20Structure))
  (bind _returnvalue (CallFunction|GetChunkSize3D))
  (bind _output_get (LocalVariables|SetNeighbourPosition (Utilities|Struct|MakeIntVector (+ (.x LocalPosition) (.x NeighbourDirection)) (+ (.y LocalPosition) (.y NeighbourDirection)) (+ (.z LocalPosition) (.z NeighbourDirection)))))
  (if (Math|Boolean|ANDBoolean (Math|Integer|InRange(Integer) (.X (Utilities|Struct|BreakIntVector _output_get)) 0 (.x _returnvalue) true false) (Math|Integer|InRange(Integer) (.Y (Utilities|Struct|BreakIntVector _output_get)) 0 (.y _returnvalue) true false) (Math|Integer|InRange(Integer) (.Z (Utilities|Struct|BreakIntVector _output_get)) 0 (.z _returnvalue) true false))
    (CallFunction|RefreshBlockVisual (LocalVariables|GetNeighbourPosition))
    (return)
    (else
      (return))))

(fn InitLog
  (Development|PrintString (Utilities|String|Append "Chunk (" (Utilities|String|ToString(Integer) (Class|VoxelChunk|GetChunkIndex)) ")  was sucessfully initialized") false)
  (return))

(fn SetBlockatLocalPositionwithInstanceHint
  (params (LocalPosition :type Int%20Vector%20Structure) (NewType :type EVoxelBlockType%20Enum :default "Air") (InstanceIndexHint :type Integer))
  (bind (_voxelblock _localblockindex _returnvalue) (CallFunction|GetBlockatLocalPosition LocalPosition))
  (LocalVariables|SetVoxelBlock _voxelblock)
  (LocalVariables|SetBlockIndex _localblockindex)
  (if _returnvalue
    (if (Utilities|Enum|Equal(Enum) (.type (LocalVariables|GetVoxelBlock)) NewType)
      (return false)
      (else
        (VoxelChunk|Editing|Helpers|RemoveBlockInstance (LocalVariables|GetBlockIndex) InstanceIndexHint)
        (VoxelChunk|Generation|Steps|Helpers|RegisterBlockbyIndex NewType (LocalVariables|GetBlockIndex))
        (Class|VoxelChunk|MarkBlockModified (LocalVariables|GetBlockIndex))
        (Class|VoxelChunk|SetDirtyFlag true)
        (CallFunction|RefreshBlockVisual LocalPosition)
        (for _array_element (Variables|VoxelChunk|Constants|GetNeighbouringDirections)
          (VoxelChunk|Editing|Helpers|RefreshNeighbourBlock LocalPosition _array_element))
        (return true)))
    (else
      (return false))))

(fn RegisterBlockbyIndex
  (params (Type :type EVoxelBlockType%20Enum :default "Air") (Index :type Integer%20%28by%20ref%29))
  (Utilities|Array|SetArrayElem (Variables|Default|GetBlocks) Index (Utilities|Struct|MakeVoxelBlock Type false))
  (return))

(fn CancelGenerationandClear
  (|CallParentFunction)
  (Class|VoxelChunk|SetGenerationState "Empty")
  (Components|InstancedStaticMesh|ClearInstances (Variables|Default|GetISM_Snow))
  (return))

(fn ApplyChunkModification
  (params (Delta :type Voxel%20Chunk%20Delta%20Structure%20%28by%20ref%29))
  (for _array_element (Utilities|Struct|BreakVoxelChunkDelta Delta)
    _))

(fn GetInstMeshComponentbyType
  (params (Type :type EVoxelBlockType%20Enum :default "Air"))
  (return (Utilities|Select :Index Type :Air 0 :Rock (Variables|Default|GetISM_Rock) :Grass (Variables|Default|GetISM_Grass) :Snow (Variables|Default|GetISM_Snow))))

(fn GetChunkSize3D
  (bind _chunksize2d (Variables|VoxelChunk|ChunkData|GetChunkSize2D))
  (return (Utilities|Struct|MakeIntVector (.x _chunksize2d) (.y _chunksize2d) (.y (Variables|VoxelChunk|ChunkData|GetChunkHeightRange)))))