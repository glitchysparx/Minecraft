(event Input|EnhancedActionEvents|EnhancedInputActionIA_Destroy
  (params (ActionValue :type Boolean) (ElapsedSeconds :type Float%20%28double-precision%29) (TriggeredSeconds :type Float%20%28double-precision%29) (InputAction :type Input%20Action%20Object%20Reference :default "/Game/Blueprints/Player/Input/Actions/IA_Destroy.IA_Destroy"))
  ;[1 1 1] Input Actions
  (:Triggered
    (CallFunction|StartMining))
  (:Canceled
    (CallFunction|StopMining :!label _label))
  (:Completed
    (goto _label)))

(event Input|EnhancedActionEvents|EnhancedInputActionIA_Build
  (params (ActionValue :type Boolean) (ElapsedSeconds :type Float%20%28double-precision%29) (TriggeredSeconds :type Float%20%28double-precision%29) (InputAction :type Input%20Action%20Object%20Reference :default "/Game/Blueprints/Player/Input/Actions/IA_Build.IA_Build"))
  ;[1 1 1] Input Actions
  (:Triggered
    (CallFunction|ProcessCrafting)))

(event EventBeginPlay
  (CallFunction|CreateHUD))

(event EventTick
  (params (DeltaSeconds :type Float%20%28single-precision%29))
  (if (Variables|Default|GetIsMiningHeld)
    (CallFunction|ProcessMining DeltaSeconds)))

(fn ConstructionScript)

(fn ProcessLineTrace
  (LocalVariables|SetStartLocation (Transformation|GetWorldLocation (Variables|Default|GetFirstPersonCameraComponent)))
  (LocalVariables|SetEndLocation (+ (* (Math|Vector|GetForwardVector (Variables|Default|GetFirstPersonCameraComponent)) (LocalVariables|GetLineTraceLength)) (LocalVariables|GetStartLocation)))
  (bind (_outhit _returnvalue) (Collision|LineTraceByChannel (LocalVariables|GetStartLocation) (LocalVariables|GetEndLocation) "TraceTypeQuery1" false 0 "None"))
  (return _outhit _returnvalue))

(fn LogHitResult
  (params (Hit :type Hit%20Result%20Structure%20%28by%20ref%29) (Condition :type Boolean))
  (bind (_bblockinghit _binitialoverlap _time _distance _location _impactpoint _normal _impactnormal _physmat _hitactor _hitcomponent _hitbonename _bonename _hititem) (Collision|BreakHitResult Hit))
  (if Condition
    (Development|PrintString (Utilities|String|Append "Line Trace Hit Log (" (Utilities|String|Append "Actor: " (Utilities|GetDisplayName _hitactor) ", Component: " (Utilities|GetDisplayName _hitcomponent) ", InstanceIndex: " (Utilities|String|ToString(Integer) _hititem)) ")") false)
    (return)
    (else
      (return))))

(fn GetMiningDuration
  (params (BlockType :type EVoxelBlockType%20Enum :default "Air"))
  (bind _miningduration (Variables|Default|GetMiningDuration))
  (bind (_value _returnvalue) (Utilities|Map|Find _miningduration BlockType))
  (return _value _returnvalue))

(fn StartMining
  (Variables|Default|SetIsMiningHeld true)
  (Default|CallOnMiningStateChanged true)
  (return))

(fn StopMining
  (Variables|Default|SetIsMiningHeld false)
  (CallFunction|ClearMiningTarget)
  (Default|CallOnMiningStateChanged false)
  (return))

(fn ProcessMining
  (params (DeltaSeconds :type Float%20%28double-precision%29))
  (bind (_outhit _returnvalue) (VoxelPlayer|Interaction|ProcessLineTrace))
  (LocalVariables|SetTraceHitResult _outhit)
  (if _returnvalue
    (LocalVariables|SetHitActor (.HitActor (Collision|BreakHitResult (LocalVariables|GetTraceHitResult))))
    (LocalVariables|SetTargetHitLocation (- (.ImpactPoint (Collision|BreakHitResult (LocalVariables|GetTraceHitResult))) (* (.ImpactNormal (Collision|BreakHitResult (LocalVariables|GetTraceHitResult))) (Variables|Default|GetTraceEndOffset))))
    (Utilities|Casting|CastToVoxelChunk (LocalVariables|GetHitActor)
      (:then
        (bind _output_get (LocalVariables|SetHitBlockPosition (Class|VoxelWorldSubsystem|BlockWorldLocationtoGlobalPosition (Subsystems|GetVoxelWorldSubsystem) (LocalVariables|GetTargetHitLocation))))
        (if (CallFunction|IsNewMiningTarget _output_get)
          (CallFunction|TrySetMiningTarget (LocalVariables|GetHitBlockPosition))
          (return)
          (else
            (bind _output_get_2 (Variables|Default|SetElapsedMiningTime (+ (Variables|Default|GetElapsedMiningTime) DeltaSeconds)))
            (if (>= _output_get_2 (Variables|Default|GetRequiredMiningTime))
              (Class|VoxelWorldSubsystem|TryDestroyBlockfromHit (Subsystems|GetVoxelWorldSubsystem) (LocalVariables|GetTraceHitResult) (Variables|Default|GetTraceEndOffset))
              (CallFunction|ClearMiningTarget)
              (return)
              (else
                (Default|CallOnMiningProgressChanged (/ (Variables|Default|GetElapsedMiningTime) (Variables|Default|GetRequiredMiningTime)))
                (return))))))
      (:CastFailed
        (CallFunction|ClearMiningTarget)
        (return)))
    (else
      (CallFunction|ClearMiningTarget)
      (return))))

(fn ClearMiningTarget
  (Variables|Default|SetHasMiningTarget false)
  (Variables|Default|SetElapsedMiningTime 0.0)
  (Default|CallOnMiningProgressChanged 0.0)
  (return))

(fn IsNewMiningTarget
  (params (BlockIndexToCheck :type Int%20Vector%20Structure))
  (bind _miningtargetblock (Variables|Default|GetMiningTargetBlock))
  (return (or (not (Variables|Default|GetHasMiningTarget)) (not (Math|Boolean|ANDBoolean (== (.x _miningtargetblock) (.x BlockIndexToCheck)) (== (.y _miningtargetblock) (.y BlockIndexToCheck)) (== (.z _miningtargetblock) (.z BlockIndexToCheck)))))))

(fn TrySetMiningTarget
  (params (NewTargetBlockIndex :type Int%20Vector%20Structure))
  (bind (_voxelblock _returnvalue) (Class|VoxelWorldSubsystem|GetBlockatGlobalPosition (Subsystems|GetVoxelWorldSubsystem) NewTargetBlockIndex))
  (LocalVariables|SetMiningBlockType (.type _voxelblock))
  (if _returnvalue
    (Variables|Default|SetMiningTargetBlock NewTargetBlockIndex)
    (Variables|Default|SetHasMiningTarget true)
    (Variables|Default|SetElapsedMiningTime 0.0)
    (Variables|Default|SetRequiredMiningTime (.TimeValue (CallFunction|GetMiningDuration (LocalVariables|GetMiningBlockType))))
    (return)
    (else
      (Development|PrintString (Utilities|String|Append "Unexpected error occured while trying to find a Block on Position: " (Utilities|String|ToString(Integer) NewTargetBlockIndex)) false)
      (return))))

(fn CreateHUD
  (bind _returnvalue (UserInterface|CreateWidget (LocalVariables|GetHUDClass) (Game|GetPlayerController 0)))
  (UserInterface|Viewport|AddtoViewport _returnvalue 0)
  (return))

(fn ProcessCrafting
  (bind _returnvalue (Subsystems|GetVoxelWorldSubsystem))
  (bind (_outhit _returnvalue_2) (VoxelPlayer|Interaction|ProcessLineTrace))
  (LocalVariables|SetTraceHitResult _outhit)
  (if _returnvalue_2
    (Class|VoxelWorldSubsystem|TryPlaceBlock _returnvalue (Class|VoxelWorldSubsystem|BlockWorldLocationtoGlobalPosition _returnvalue (+ (.ImpactPoint (Collision|BreakHitResult (LocalVariables|GetTraceHitResult))) (* (.ImpactNormal (Collision|BreakHitResult (LocalVariables|GetTraceHitResult))) (Variables|Default|GetTraceEndOffset)))) "Rock")
    (return)
    (else
      (return))))