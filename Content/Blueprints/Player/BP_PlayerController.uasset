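; Player controller that covers voxel world generation with a loading screen and hands control to the player once the world is ready.
; On BeginPlay it binds to the VoxelWorldSubsystem's initial-world-ready event, shows the loading widget and disables character input.
; When generation finishes, it teleports the character to a safe spawn location from the subsystem, removes the loading screen, restores input and creates the HUD.
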(event EventBeginPlay
  (EventDispatchers|BindEventtoOnInitialWorldReady (Subsystems|GetVoxelWorldSubsystem) (EventDispatchers|CreateEvent :!event OnWorldGenerationFinished))
  (CallFunction|OnWorldGenerationStarted))

(fn ConstructionScript)

(fn OnWorldGenerationStarted
  (bind _returnvalue (UserInterface|CreateWidget "/Game/Blueprints/UI/WB_LoadingScreen.WB_LoadingScreen_C" self))
  (bind _output_get (Variables|Default|SetLoadingScreen _returnvalue))
  (Utilities|IsValid _output_get
    (:Is%20Valid
      (UserInterface|Viewport|AddtoViewport (Variables|Default|GetLoadingScreen) 0)
      (Input|DisableInput (Game|GetPlayerCharacter 0) self)
      (return))
    (:Is%20Not%20Valid
      (Development|PrintString "Error: Failed to create Loading Screen widget" false)
      (return))))

(fn OnWorldGenerationFinished
  (Utilities|IsValid (Variables|Default|GetLoadingScreen)
    (:Is%20Valid
      (Transformation|SetActorLocation (Game|GetPlayerCharacter 0) (Class|VoxelWorldSubsystem|FindSafePlayerSpawnLocation (Subsystems|GetVoxelWorldSubsystem)) false true)
      (Widget|RemovefromParent (Variables|Default|GetLoadingScreen))
      (Input|EnableInput (Game|GetPlayerCharacter 0) self)
      (CallFunction|CreateHUD)
      (return))
    (:Is%20Not%20Valid
      (return))))

(fn CreateHUD
  (bind _returnvalue (UserInterface|CreateWidget (LocalVariables|GetHUDClass) self))
  (UserInterface|Viewport|AddtoViewport _returnvalue 0)
  (return))